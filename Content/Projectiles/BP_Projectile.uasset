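; Projectile actor that flies at its Speed value and hits fighters, with its box collision ignoring the Emitter that fired it.
; The construction script feeds Speed into the projectile movement component as initial speed.
; On hitting a BP_Fighter it passes Speed to HitByProjectile, fires OnProjectileImpact, plays lightning and explosion effects, then destroys itself.
; Hits on anything other than a fighter trigger none of this, including the destroy.
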(event `self.ReceiveBeginPlay`
  (`PrimitiveComponent.IgnoreActorWhenMoving` (`self.Box Colision`) (`self.emitter`) true))

(event `self.Box Colision.OnComponentHit`
  (params (HitComponent :type "PrimitiveComponent Object Reference") (OtherActor :type "Actor Object Reference") (OtherComp :type "PrimitiveComponent Object Reference") (NormalImpulse :type "Vector Structure") (Hit :type "HitResult Structure (by ref)"))
  (bind (_bblockinghit _binitialoverlap _time _distance _location) (`GameplayStatics.BreakHitResult` Hit))
  (bind _asbp_fighter (cast `/Game/Blueprints/BP_Fighter` OtherActor))
  (`/Game/Blueprints/BP_Fighter.HitByProjectile` _asbp_fighter (`self.speed`))
  (`self.onProjectileImpact` null Hit)
  (`GameplayStatics.SpawnEmitterAtLocation` "/Game/InfinityBladeEffects/Effects/FX_Monsters/FX_Monster_Gruntling/Lightning/P_Gruntling_Lightning_Impact_01.P_Gruntling_Lightning_Impact_01" _location)
  (`GameplayStatics.PlaySoundAtLocation` "/Game/StarterContent/Audio/Explosion01.Explosion01" _location (struct) 0.5 1.0 0.0 null null null null)
  (`self.K2_DestroyActor`))

(fn `UserConstructionScript`
  (set `ProjectileMovementComponent.InitialSpeed` (`self.speed`) (`self.ProjectileMovement`)))